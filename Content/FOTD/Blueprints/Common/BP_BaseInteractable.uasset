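; Base interactable actor that shows a fading hint widget and gives its contents to the player's inventory.
; Sphere overlap with the first-person character creates or removes the widget, while trace and ShowHint events also drive it, tracked by HintVisible.
; PickupItem adds each Contents entry to the player, calling DestroyActor inside the loop when SingleUse is set.
; Getters expose locked and interactable state; GetContents returns nothing.
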(event `self.Sphere.OnComponentBeginOverlap`
  (params (OverlappedComponent :type "PrimitiveComponent Object Reference") (OtherActor :type "Actor Object Reference") (OtherComp :type "PrimitiveComponent Object Reference") (OtherBodyIndex :type Integer) (bFromSweep :type Boolean) (SweepResult :type "HitResult Structure (by ref)"))
  (bind _widget (`self.Widget`))
  ; Begin OverlapEvent
  (cast `/Game/FOTD/Blueprints/Character/BP_FirstPersonCharacter` OtherActor)
  (if (`self.Interactable`)
    (bind _returnvalue (`|CreateWidget` "/Game/FOTD/Blueprints/UI/InteractableUI.InteractableUI_C"))
    (bind _output_get (set `self.InteractionWidget` _returnvalue))
    (`WidgetComponent.SetWidget` _widget _output_get)
    (`SceneComponent.SetVisibility` _widget true false)
    (bind _interactionwidget (`self.InteractionWidget`)
      (:`then`
        (if (not (`self.HintVisible`))
          (`UserWidget.PlayAnimationForward` _interactionwidget (`/Game/FOTD/Blueprints/UI/InteractableUI.Fade` _interactionwidget) 1.5 false)
          (set `self.HintVisible` true)))
      (:`else`))))

(event `self.Sphere.OnComponentEndOverlap`
  (params (OverlappedComponent :type "PrimitiveComponent Object Reference") (OtherActor :type "Actor Object Reference") (OtherComp :type "PrimitiveComponent Object Reference") (OtherBodyIndex :type Integer))
  ; End Overlap Event
  (cast `/Game/FOTD/Blueprints/Character/BP_FirstPersonCharacter` OtherActor)
  (if (`self.Interactable`)
    (bind _interactionwidget (`self.InteractionWidget`)
      (:`then`
        (if (`self.HintVisible`)
          (`UserWidget.PlayAnimationReverse` _interactionwidget (`/Game/FOTD/Blueprints/UI/InteractableUI.Fade` _interactionwidget) 1.0 false)
          (set `self.HintVisible` false))
        (`KismetSystemLibrary.Delay` 0.2)
        (`Widget.RemoveFromParent` (`self.InteractionWidget`))
        (set `self.InteractionWidget` null)
        (`SceneComponent.SetVisibility` (`self.Widget`) false false))
      (:`else`))))

(event `/Game/FOTD/Blueprints/Common/BPI_Interactable.Can Receive Trace`
  (params (CanInteract :type Boolean))
  ; TraceEvent
  (if (`self.Interactable`)
    (if CanInteract
      (bind _interactionwidget (`self.InteractionWidget`)
        (:`then`
          (if (`self.HintVisible`)
            (`UserWidget.PlayAnimation` _interactionwidget (`/Game/FOTD/Blueprints/UI/InteractableUI.Fade` _interactionwidget) 0.0 1 "Forward" 1.5 false)
            (set `self.HintVisible` true)))
        (:`else`))
      (else
        (bind _interactionwidget_2 (`self.InteractionWidget` :!label _label)
          (:`then`
            (if (`self.HintVisible`)
              (`UserWidget.PlayAnimation` _interactionwidget_2 (`/Game/FOTD/Blueprints/UI/InteractableUI.Fade` _interactionwidget_2) 0.0 1 "Reverse" 1.5 false)
              (set `self.HintVisible` false)))
          (:`else`))))
    (else
      (goto _label))))

(event `/Game/FOTD/Blueprints/Common/BPI_Interactable.ShowHint`
  (params (ShowHint :type Boolean))
  (bind _widget (`self.Widget`))
  ; ShowHint
  (if ShowHint
    (bind _returnvalue (`|CreateWidget` "/Game/FOTD/Blueprints/UI/InteractableUI.InteractableUI_C"))
    (bind _output_get (set `self.InteractionWidget` _returnvalue))
    (`WidgetComponent.SetWidget` _widget _output_get)
    (`SceneComponent.SetVisibility` _widget true false)
    (bind _interactionwidget (`self.InteractionWidget`)
      (:`then`
        (if (not (`self.HintVisible`))
          (`UserWidget.PlayAnimationForward` _interactionwidget (`/Game/FOTD/Blueprints/UI/InteractableUI.Fade` _interactionwidget) 1.5 false)
          (set `self.HintVisible` true)))
      (:`else`))
    (elif (`self.Interactable`)
      (if (`self.HintVisible`)
        (`Widget.RemoveFromParent` (`self.InteractionWidget`))
        (set `self.InteractionWidget` null)
        (`SceneComponent.SetVisibility` (`self.Widget`) false false)
        (set `self.HintVisible` false)))))

(event `/Game/FOTD/Blueprints/Common/BPI_Interactable.PickupItem`
  (params (Player :type "/Game/FOTD/Blueprints/Character/BP_FirstPersonCharacter Object Reference"))
  (for _array_element (`self.Contents`)
    (`/Game/FOTD/Blueprints/Character/BP_FirstPersonCharacter.AddItemToInventory` Player _array_element)
    (message `/Game/FOTD/Blueprints/Common/BPI_Interactable.RemoveItem` self _array_element)
    (if (`self.SingleUse`)
      (`self.K2_DestroyActor`))))

(fn `GetContents`
  (returns (Contents :type "Array of /Game/FOTD/Blueprints/Common/S_BaseItem Structure"))
  (return))

(fn `IsInteractable`
  (returns (IsInteractable :type Boolean))
  (return (`self.Interactable`)))

(fn `isLocked`
  (returns (locked :type Boolean))
  (return (`self.Locked`)))

(fn `UserConstructionScript`)