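; BP_BaseDoor is an interactable door that opens, then closes itself, and can be locked behind an inventory key.
; Timelines move the door mesh, suspending interaction and its hint during the cycle.
; On a locked door, a player's interaction searches their inventory for ItemId, either unlocking it without opening or playing a locked sound.
; Tick enables the NavLinkProxy smart link only while the door is unlocked.
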(event `self.ReceiveTick`
  (params (DeltaSeconds :type "Float (single-precision)"))
  (bind _navlinkproxy (`self.NavLinkProxy`))
  ;[1 1 1] Enable Navigation
  (`/Engine/EditorBlueprintResources/StandardMacros.IsValid` _navlinkproxy
    (:`Is Valid`
      (bind _locked (`self.isLocked`))
      (`NavLinkProxy.SetSmartLinkEnabled` _navlinkproxy (not _locked)))))

(event `/Game/FOTD/Blueprints/Common/BPI_Interactable.Interact`
  (params (Actor :type "/Game/FOTD/Blueprints/Character/BP_FirstPersonCharacter Object Reference"))
  ;[1 1 1] Interaction
  (if (`self.Interactable`)
    (if (`self.Locked`)
      (if (`self.ActorHasTag` Actor "Player")
        (bind _keyfound (`self.CheckKey` Actor))
        (if (not _keyfound)
          (`GameplayStatics.PlaySound2D` "/Game/FOTD/Soundbites/324601__univ_lyon3__koudsi_linda_2015_2016_lockeddoor.324601__univ_lyon3__koudsi_linda_2015_2016_lockeddoor" 1.0 1.0 0.0 null null false)))
      (elif (not (`self.opening`))
        (bind (_direction _dooropen) (`Timeline|OpenDoor` :!via `PlayFromStart`)
          (:`Update`
            (`SceneComponent.K2_SetRelativeLocation` (`self.Door`) _dooropen false false)
            (set `self.opening` true)
            (`/Game/FOTD/Blueprints/Common/BPI_Interactable.ShowHint` false)
            (set `self.Interactable` false))
          (:`Finished`
            (bind (_direction_2 _dooropen_2) (`Timeline|CloseDoor` :!via `ReverseFromEnd`)
              (:`Update`
                (`SceneComponent.K2_SetRelativeLocation` (`self.Door`) _dooropen_2 false false))
              (:`Finished`
                (set `self.opening` false)
                (set `self.Interactable` true)
                (if (`PrimitiveComponent.IsOverlappingActor` (`self.Sphere`) Actor)
                  (`/Game/FOTD/Blueprints/Common/BPI_Interactable.ShowHint` true))))))))))

(fn `CheckKey`
  (params (Player :type "Object Object Reference"))
  (returns (KeyFound :type Boolean))
  (locals (ItemFound :type Boolean :default false))
  (bind _itemfound (`local.ItemFound`))
  (bind _asbp_first_person_character (cast `/Game/FOTD/Blueprints/Character/BP_FirstPersonCharacter` Player)
    (:`then`
      (bind _itemfound_2 (`/Game/FOTD/Blueprints/Character/BP_FirstPersonCharacter.FindItemInInventory` _asbp_first_person_character (`self.Item Id`)))
      (set `local.ItemFound` _itemfound_2))
    (:`CastFailed`
      (set `local.ItemFound` false)))
  (set `self.Locked` (not _itemfound))
  (return _itemfound))

(fn `IsInteractable`
  (returns (IsInteractable :type Boolean))
  (return false))

(fn `UserConstructionScript`)