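; BP_Box is an interactable box that opens and passes the interacting actor to PickupItem.
; When interactable, unlocked and closed, it plays the box animation once, hides its hint and disables further interaction.
; If it is already open and still interactable, Interact only clears IsOpen, with no animation.
; RemoveItem removes an item from the GetContents result, though GetContents has an empty return here.
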(event `/Game/FOTD/Blueprints/Common/BPI_Interactable.Interact`
  (params (Actor :type "/Game/FOTD/Blueprints/Character/BP_FirstPersonCharacter Object Reference"))
  (if (`self.Interactable`)
    (if (`self.Locked`)
      _
      (elif (`self.isOpen`)
        (set `self.isOpen` false)
        (else
          (set `self.isOpen` true)
          (`SkeletalMeshComponent.PlayAnimation` (`self.Box_0`) "/Game/FOTD/Models/Box/BoxAnim.BoxAnim" false)
          (`/Game/FOTD/Blueprints/Common/BPI_Interactable.ShowHint` false)
          (set `self.Interactable` false)
          (`/Game/FOTD/Blueprints/Common/BPI_Interactable.PickupItem` Actor))))))

(event `/Game/FOTD/Blueprints/Common/BPI_Interactable.RemoveItem`
  (params (Item :type "/Game/FOTD/Blueprints/Common/S_BaseItem Structure"))
  (bind _contents (`/Game/FOTD/Blueprints/Common/BPI_Interactable.GetContents`))
  (`KismetArrayLibrary.Array_RemoveItem` _contents Item))

(fn `GetContents`
  (returns (Contents :type "Array of /Game/FOTD/Blueprints/Common/S_BaseItem Structure"))
  (return))

(fn `UserConstructionScript`)